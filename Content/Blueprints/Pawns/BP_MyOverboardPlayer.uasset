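; Player pawn for an overboard-style board that tilts to follow the slope of the ground beneath it.
; Each Tick, a downward line trace from BoardGroundDetector checks for ground while that component is active.
; On a hit, a second trace from BoardContainer yields slope pitch and roll, which RInterpTo blends into the board's rotation, keeping its yaw.
; On a miss, the detector deactivates, and nothing here reactivates it.
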(event `self.ReceiveTick`
  (params (DeltaSeconds :type "Float (single-precision)"))
  (bind _isonground (`self.IsOnGround`))
  (if _isonground
    (`self.SetBoardFollowGround` DeltaSeconds)
    (else
      (`ActorComponent.Deactivate` (`self.boardGroundDetector_`)))))

(fn `IsOnGround`
  (returns (IsOnGround :type Boolean))
  (bind _boardgrounddetector_ (`self.boardGroundDetector_`))
  (bind _returnvalue (`SceneComponent.K2_GetComponentLocation` _boardgrounddetector_))
  (if (`ActorComponent.IsActive` _boardgrounddetector_)
    (bind (_outhit _returnvalue_2) (`KismetSystemLibrary.LineTraceSingle` _returnvalue (- _returnvalue (* (`SceneComponent.GetUpVector` _boardgrounddetector_) 100)) "TraceTypeQuery1"))
    (return _returnvalue_2)))

(fn `SetBoardFollowGround`
  (params (DeltaTime :type "Float (double-precision)"))
  (bind _boardcontainer_ (`self.boardContainer_`))
  (bind _returnvalue (`SceneComponent.K2_GetComponentRotation` (`self.boardContainer_`)))
  (bind _returnvalue_2 (`SceneComponent.K2_GetComponentLocation` _boardcontainer_))
  (bind _outhit (`KismetSystemLibrary.LineTraceSingle` _returnvalue_2 (- _returnvalue_2 (* (`SceneComponent.GetUpVector` _boardcontainer_) 100)) "TraceTypeQuery1"))
  (bind (_outslopepitchdegreeangle _outsloperolldegreeangle) (`KismetMathLibrary.GetSlopeDegreeAngles` (`self.GetActorRightVector`) (`.ImpactNormal` (`GameplayStatics.BreakHitResult` _outhit)) (`self.GetActorUpVector`)))
  (bind _result (`/Engine/EditorBlueprintResources/StandardMacros.NegateFloat` _outsloperolldegreeangle)
    (:`  `
      (`SceneComponent.K2_SetWorldRotation` (`self.boardContainer_`) (`KismetMathLibrary.RInterpTo` _returnvalue (`KismetMathLibrary.MakeRotator` _result _outslopepitchdegreeangle (.yaw _returnvalue)) DeltaTime) false false))))

(fn `UserConstructionScript`)