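; Overboard player Blueprint that tilts its board to follow the slope of the ground beneath it.
; Each Tick, IsOnGround traces down from BoardGroundDetector while that component is active.
; On a hit, SetBoardFollowGround traces from BoardContainer and turns the impact normal into pitch and roll through RInterpTo, keeping yaw.
; A miss deactivates the detector, and nothing here reactivates it.
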(event `self.ReceiveTick`
  (params (DeltaSeconds :type "Float (single-precision)"))
  (bind _isonground (`self.IsOnGround`))
  (if _isonground
    (`self.SetBoardFollowGround` DeltaSeconds)
    (else
      (`ActorComponent.Deactivate` (`self._boardGroundDetector`)))))

(fn `IsOnGround`
  (returns (IsOnGround :type Boolean))
  (bind __boardgrounddetector (`self._boardGroundDetector`))
  (bind _returnvalue (`SceneComponent.K2_GetComponentLocation` __boardgrounddetector))
  (if (`ActorComponent.IsActive` __boardgrounddetector)
    (bind (_outhit _returnvalue_2) (`KismetSystemLibrary.LineTraceSingle` _returnvalue (- _returnvalue (* (`SceneComponent.GetUpVector` __boardgrounddetector) 100)) "TraceTypeQuery1"))
    (return _returnvalue_2)))

(fn `SetBoardFollowGround`
  (params (DeltaTime :type "Float (double-precision)"))
  (bind __boardcontainer (`self._boardContainer`))
  (bind _returnvalue (`SceneComponent.K2_GetComponentRotation` (`self._boardContainer`)))
  (bind _returnvalue_2 (`SceneComponent.K2_GetComponentLocation` __boardcontainer))
  (bind _outhit (`KismetSystemLibrary.LineTraceSingle` _returnvalue_2 (- _returnvalue_2 (* (`SceneComponent.GetUpVector` __boardcontainer) 100)) "TraceTypeQuery1"))
  (bind (_outslopepitchdegreeangle _outsloperolldegreeangle) (`KismetMathLibrary.GetSlopeDegreeAngles` (`self.GetActorRightVector`) (`.ImpactNormal` (`GameplayStatics.BreakHitResult` _outhit)) (`self.GetActorUpVector`)))
  (bind _result (`/Engine/EditorBlueprintResources/StandardMacros.NegateFloat` _outsloperolldegreeangle)
    (:`  `
      (`SceneComponent.K2_SetWorldRotation` (`self._boardContainer`) (`KismetMathLibrary.RInterpTo` _returnvalue (`KismetMathLibrary.MakeRotator` _result _outslopepitchdegreeangle (.yaw _returnvalue)) DeltaTime) false false))))

(fn `UserConstructionScript`)